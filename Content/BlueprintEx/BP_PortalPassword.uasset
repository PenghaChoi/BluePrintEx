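; BP_PortalPassword is a password puzzle actor that shows its Sphere when a set of counters matches a stored code.
; On BeginPlay it hides the Sphere and binds a callback to the F-click event dispatcher of each object in the Counts array.
; FuncPressFClick prints a debug string and sets Sphere visibility from IsAllBox9, which compares each Count to the Password entry at the same index.
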(event EventBeginPlay
  (Rendering|SetVisibility (Variables|Default|GetSphere) false false)
  (for _array_element (Variables|Default|GetCounts)
    (EventDispatchers|BindEventtoEventDispatcherFClick _array_element (EventDispatchers|CreateEvent :!event FuncPressFClick))))

(fn ConstructionScript)

(fn FuncPressFClick
  (Development|PrintString "PressFClick")
  (Rendering|SetVisibility (Variables|Default|GetSphere) (CallFunction|IsAllBox9) false))

(fn IsAllBox9
  (for (_array_element _array_index) (Variables|Default|GetCounts)
    (if (not (== (Variables|/Game/BlueprintEx/BP_CountBox.BP_CountBox_C|GetCount _array_element) (Utilities|Array|Get(acopy) (Variables|Default|GetPassword) _array_index)))
      (return false)))
  (return true))