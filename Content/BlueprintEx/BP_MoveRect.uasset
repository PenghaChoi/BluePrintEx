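; Example actor that moves its Cube around a rectangular path in the local X-Z plane while switched on.
; BeginPlay binds to the Switch's toggle dispatcher, with EventSwitchToggle setting IsPlay to gate Tick.
; Tick runs a MoveType state machine through Right, Up, Left and Down, changing state when PosX or PosZ passes a limit.
; Each move function applies a fixed per-frame step to the Cube's relative location, so speed depends on frame rate.
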(event EventTick
  (params (DeltaSeconds :type Float%20%28single-precision%29))
  (if (Variables|Default|GetIsPlay)
    (switch Utilities|FlowControl|Switch|SwitchonEN_MoveType (Variables|Default|GetMoveType)
      (:NewEnumerator0
        (CallFunction|MoveRight)
        (if (> (Variables|Default|GetPosX) 1e+02)
          (Variables|Default|SetMoveType "NewEnumerator1")))
      (:NewEnumerator1
        (CallFunction|MoveUp)
        (if (> (Variables|Default|GetPosZ) 1e+02)
          (Variables|Default|SetMoveType "NewEnumerator2")))
      (:NewEnumerator2
        (CallFunction|MoveLeft)
        (if (< (Variables|Default|GetPosX) 0.0)
          (Variables|Default|SetMoveType "NewEnumerator3")))
      (:NewEnumerator3
        (CallFunction|MoveDown)
        (if (< (Variables|Default|GetPosZ) 0.0)
          (Variables|Default|SetMoveType "NewEnumerator0"))))))

(event EventBeginPlay
  (EventDispatchers|BindEventtoEventDispatcherToggle (Variables|Default|GetSwitch) (EventDispatchers|CreateEvent :!event EventSwitchToggle)))

(fn ConstructionScript)

(fn MoveRight
  (Variables|Default|SetPosX (+ (Variables|Default|GetPosX) 1e+01))
  (Transformation|SetRelativeLocation (Variables|Default|GetCube) (Math|Vector|MakeVector (Variables|Default|GetPosX) 0.0 (Variables|Default|GetPosZ)) false false))

(fn MoveUp
  (Variables|Default|SetPosZ (+ (Variables|Default|GetPosZ) 1e+01))
  (Transformation|SetRelativeLocation (Variables|Default|GetCube) (Math|Vector|MakeVector (Variables|Default|GetPosX) 0.0 (Variables|Default|GetPosZ)) false false))

(fn MoveLeft
  (Variables|Default|SetPosX (- (Variables|Default|GetPosX) 1e+01))
  (Transformation|SetRelativeLocation (Variables|Default|GetCube) (Math|Vector|MakeVector (Variables|Default|GetPosX) 0.0 (Variables|Default|GetPosZ)) false false))

(fn MoveDown
  (Variables|Default|SetPosZ (- (Variables|Default|GetPosZ) 1e+01))
  (Transformation|SetRelativeLocation (Variables|Default|GetCube) (Math|Vector|MakeVector (Variables|Default|GetPosX) 0.0 (Variables|Default|GetPosZ)) false false))

(fn EventSwitchToggle
  (params (toggle :type Boolean))
  (Variables|Default|SetIsPlay toggle))